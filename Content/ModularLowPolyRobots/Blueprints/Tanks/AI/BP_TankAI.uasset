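; AI controller for the robot tank that chases the player and shoots while it perceives them.
; On possessing a BP_Tank it runs BT_Tank, and AI Perception updates the "CanSee?" blackboard key and starts or stops the tank's firing.
; Movement is also driven outside the tree: a looping timer moves toward the player regardless of sensing, and Tick pursues the last pawn seen or heard through Pawn Sensing.
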(event `self.ReceiveBeginPlay`
  (`KismetSystemLibrary.K2_SetTimerDelegate` (delegate `Buscar Al Jugador`) 1.0 true))

(event `Buscar Al Jugador`
  (`|AIMoveTo` (`self.K2_GetPawn`) (0.0 0.0 0.0) (`GameplayStatics.GetPlayerPawn` 0) 200.0
    (:`OnFail`
      (`KismetSystemLibrary.PrintString` "AI ERROR" true true (struct :`R` 0.633333 :`B` 0.026136 :`A` 1.0)))))

(event `self.ReceivePossess`
  (params (PossessedPawn :type "Pawn Object Reference"))
  ;[0.4871 0.6816 1] On Possess
  (cast `/Game/ModularLowPolyRobots/Blueprints/Tanks/BP_Tank` PossessedPawn)
  (`self.RunBehaviorTree` "/Game/ModularLowPolyRobots/Blueprints/Tanks/AI/BT_Tank.BT_Tank"))

(event `self.PawnSensing.OnSeePawn`
  (params (Pawn :type "Pawn Object Reference"))
  ;[0.4292 1 0.5452] Pawn Sensing
  (set `self.Target` Pawn)
  (`self.MoveToActor` Pawn 200.0 true true true null))

(event `self.PawnSensing.OnHearNoise`
  (params (Instigator :type "Pawn Object Reference") (Location :type "Vector Structure (by ref)") (Volume :type "Float (single-precision)"))
  ;[0.4292 1 0.5452] Pawn Sensing
  (set `self.Target` Instigator)
  (`self.MoveToActor` Instigator 200.0 true true true null))

(event `self.AIPerception.OnTargetPerceptionUpdated`
  (params (Actor :type "Actor Object Reference") (Stimulus :type "AIStimulus Structure"))
  (bind (_age _expirationage _strength _stimuluslocation _receiverlocation _tag _bsuccessfullysensed) (break `AIStimulus` Stimulus))
  (bind _returnvalue (`self.K2_GetPawn`))
  ;[0.4871 0.6816 1] On Possess
  (cast `/Game/ThirdPersonBP/Blueprints/ThirdPersonCharacter` Actor)
  (`BlackboardComponent.SetValueAsBool` (`AIBlueprintHelperLibrary.GetBlackboard` null) "CanSee?" _bsuccessfullysensed)
  (if _bsuccessfullysensed
    (bind _asbp_tank (cast `/Game/ModularLowPolyRobots/Blueprints/Tanks/BP_Tank` _returnvalue))
    (`/Game/ModularLowPolyRobots/Blueprints/Tanks/BP_Tank.Empezar a Disparar` _asbp_tank)
    (else
      (bind _asbp_tank_2 (cast `/Game/ModularLowPolyRobots/Blueprints/Tanks/BP_Tank` _returnvalue))
      (`/Game/ModularLowPolyRobots/Blueprints/Tanks/BP_Tank.Dejar De Disparar` _asbp_tank_2))))

(event `self.ReceiveTick`
  (params (DeltaSeconds :type "Float (single-precision)"))
  (bind _target (`self.Target`))
  (`/Engine/EditorBlueprintResources/StandardMacros.IsValid` _target
    (:`Is Valid`
      (`self.MoveToActor` _target 200.0 true true true null))))

(fn `UserConstructionScript`)