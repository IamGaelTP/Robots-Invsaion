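; Tank entity that fires lasers from two muzzle points and loses health when damaged.
; Start and stop events run a looping timer on ShootTime, with each shot spawning two owned Laser actors and playing a sound.
; Construction script loads Health, Damage and Speed from the Tank1 row of DT_Tanks.
; AnyDamage subtracts health only when the damage causer passes an equality check, with no death handling here.
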(event `Empezar a Disparar`
  ;[0.9641 0.4503 1] Shoot
  (`self.Disparar`)
  (`KismetSystemLibrary.K2_SetTimer` null "Disparar" (`self.shootTime`) true))

(event `Dejar De Disparar`
  ;[0.9641 0.4503 1] Shoot
  (`KismetSystemLibrary.K2_ClearTimer` null "Disparar"))

(event `Disparar`
  ;[0.9641 0.4503 1] Shoot
  (`|ExecutionSequence`
    (:`then_0`
      (`|SpawnActorFromClass` (`self.Laser`) (`SceneComponent.K2_GetComponentToWorld` (`self.Direction1`)) "Undefined" "OverrideRootScale" self null))
    (:`then_1`
      (`|SpawnActorFromClass` (`self.Laser`) (`SceneComponent.K2_GetComponentToWorld` (`self.Direction`)) "Undefined" "OverrideRootScale" self null))
    (:`then_2`
      (`GameplayStatics.PlaySoundAtLocation` null (`self.K2_GetActorLocation`) (struct) 1.0 1.0 0.0 null null null))))

(event `self.ReceiveAnyDamage`
  (params (Damage :type "Float (single-precision)") (DamageType :type "DamageType Object Reference") (InstigatedBy :type "Controller Object Reference") (DamageCauser :type "Actor Object Reference"))
  ;[1 0.4023 0.3565] On Damage
  (if (== DamageCauser null)
    (set `self.health` (`KismetMathLibrary.FTrunc` (- (`KismetMathLibrary.Conv_IntToDouble` (`self.health`)) Damage)))))

(fn `UserConstructionScript`
  ;[0.5441 1 0.5688] Set Values
  (bind _returnvalue (`|GetDataTableRow` "/Game/ModularLowPolyRobots/Blueprints/Tanks/DT_Tanks.DT_Tanks" "Tank1")
    (:`then`
      (`|ExecutionSequence`
        (:`then_0`
          (bind (_health _damage _speed) (break `/Game/ModularLowPolyRobots/Blueprints/Tanks/ST_Tanks` _returnvalue))
          (set `self.health` _health))
        (:`then_1`
          (set `self.damage` _damage))
        (:`then_2`
          (set `self.speed` _speed))))))