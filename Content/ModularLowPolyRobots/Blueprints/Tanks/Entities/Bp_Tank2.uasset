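; Bp_Tank2 is the second tank variant among the modular low-poly robots, configured entirely in its construction script.
; It reads Health, Damage and Speed from the Tank2 row of the DT_Tanks data table.
; It also sets BP_Laser2 as its laser and registers Direction1 as a bullet spawn point.
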(fn `UserConstructionScript`
  (`|ExecutionSequence`
    (:`then_0`
      ;[0.5441 1 0.5688] Set Values
      (bind _returnvalue (`|GetDataTableRow` "/Game/ModularLowPolyRobots/Blueprints/Tanks/DT_Tanks.DT_Tanks" "Tank2")
        (:`then`
          (`|ExecutionSequence`
            (:`then_0`
              (bind (_health _damage _speed) (break `/Game/ModularLowPolyRobots/Blueprints/Tanks/ST_Tanks` _returnvalue))
              (set `self.health` _health))
            (:`then_1`
              (set `self.damage` _damage))
            (:`then_2`
              (set `self.speed` _speed))))))
    (:`then_1`
      (set `self.Laser` "/Game/ModularLowPolyRobots/Blueprints/Tanks/Bullets/BP_Laser2.BP_Laser2_C"))
    (:`then_2`
      (`KismetArrayLibrary.Array_AddUnique` (`self.bulletSpawn`) (`self.Direction1`)))))