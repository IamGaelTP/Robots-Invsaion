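; Tank Blueprint from the modular low-poly robots content that fires on a repeating timer.
; The construction script loads Health, Damage and Speed from the Tank1 row of DT_Tanks.
; EmpezaraDisparar fires immediately and starts a looping timer at ShootTime intervals, which DejarDeDisparar clears.
; Each Disparar call spawns two actors, both at the Direction1 transform, and plays a sound at the tank's location.
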(event `self.ReceiveTick`
  (params (DeltaSeconds :type "Float (single-precision)")))

(event `Empezar a Disparar`
  (`self.Disparar`)
  (`KismetSystemLibrary.K2_SetTimer` null "Disparar" (`self.shootTime`) true))

(event `Dejar De Disparar`
  (`KismetSystemLibrary.K2_ClearTimer` null "Disparar"))

(event `Disparar`
  (bind _returnvalue (`SceneComponent.K2_GetComponentToWorld` (`self.Direction1`)))
  (`|ExecutionSequence`
    (:`then_0`
      (`|SpawnActorFromClass` "/Game/ModularLowPolyRobots/Blueprints/Tanks/Bullets/BP_Laser.BP_Laser_C" _returnvalue "Undefined" "OverrideRootScale" null null))
    (:`then_1`
      (`|SpawnActorFromClass` "/Game/ModularLowPolyRobots/Blueprints/Tanks/Bullets/BP_Laser.BP_Laser_C" _returnvalue "Undefined" "OverrideRootScale" null null))
    (:`then_2`
      (`GameplayStatics.PlaySoundAtLocation` null (`self.K2_GetActorLocation`) (struct) 1.0 1.0 0.0 null null null))))

(fn `UserConstructionScript`
  ;[0.5441 1 0.5688] Set Values
  (bind _returnvalue (`|GetDataTableRow` "/Game/ModularLowPolyRobots/Blueprints/Tanks/DT_Tanks.DT_Tanks" "Tank1")
    (:`then`
      (`|ExecutionSequence`
        (:`then_0`
          (bind (_health _damage _speed) (break `/Game/ModularLowPolyRobots/Blueprints/Tanks/ST_Tanks` _returnvalue))
          (set `self.health` _health))
        (:`then_1`
          (set `self.damage` _damage))
        (:`then_2`
          (set `self.speed` _speed))))))