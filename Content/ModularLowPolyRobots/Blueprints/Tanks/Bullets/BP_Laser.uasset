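; BP_Laser is a laser projectile fired by BP_Tank enemies in the Modular Low Poly Robots pack.
; It destroys itself after five seconds, on a hit, or on any actor overlap.
; When it overlaps the player's ThirdPersonCharacter, it first applies damage taken from its owning tank's Damage value, with the tank's controller as instigator.
; A failed cast of the owner or player stops that path before destruction.
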(event `self.ReceiveBeginPlay`
  (`KismetSystemLibrary.Delay` 5.0)
  (`self.K2_DestroyActor`))

(event `self.ReceiveHit`
  (params (MyComp :type "PrimitiveComponent Object Reference") (Other :type "Actor Object Reference") (OtherComp :type "PrimitiveComponent Object Reference") (bSelfMoved :type Boolean) (HitLocation :type "Vector Structure") (HitNormal :type "Vector Structure") (NormalImpulse :type "Vector Structure") (Hit :type "HitResult Structure (by ref)"))
  (`self.K2_DestroyActor`))

(event `self.ReceiveActorBeginOverlap`
  (params (OtherActor :type "Actor Object Reference"))
  (if (== OtherActor (`GameplayStatics.GetPlayerCharacter` 0))
    (bind _asbp_tank (cast `/Game/ModularLowPolyRobots/Blueprints/Tanks/Entities/BP_Tank` (`self.GetOwner`)))
    (bind _asthird_person_character (cast `/Game/ThirdPersonBP/Blueprints/ThirdPersonCharacter` (`GameplayStatics.GetPlayerCharacter` 0)))
    (`GameplayStatics.ApplyDamage` _asthird_person_character (`KismetMathLibrary.Conv_IntToDouble` (`/Game/ModularLowPolyRobots/Blueprints/Tanks/Entities/BP_Tank.damage` _asbp_tank)) (`Pawn.GetController` _asbp_tank) self "/Script/Engine.DamageType"))
  (`self.K2_DestroyActor`))

(fn `UserConstructionScript`)